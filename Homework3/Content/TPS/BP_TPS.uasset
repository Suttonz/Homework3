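; BP_TPS is a third-person player character handling camera look, yaw-relative movement, crouch, sprint and weapon aiming.
; Input flags coordinate the states, with right mouse playing standing or crouched weapon-hold montages.
; Shift raises walk speed, blocks move input and opens a Tick-fed gate that auto-runs forward unless crouched, while Tick also stops aim montages.
; Prone only sets a flag, and releasing aim never clears its flag.
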(event Custom|Stop%20aiming%20while%20sprinting
  ;[1 1 1] Stop Aiming animation when start sprinting
  (if (Variables|Default|GetSprintButtonPressed)
    (Animation|StopAnimMontage "/Game/TPS/M_TPS_WeaponHoldNormal.M_TPS_WeaponHoldNormal")
    (if (Variables|Default|GetCrouchButtonPressed)
      (Animation|StopAnimMontage "/Game/TPS/M_TPS_WeaponHoldCrouch.M_TPS_WeaponHoldCrouch"))))

(event Custom|Sprint
  ;[1 1 1] Sprint
  (if (not (Variables|Default|GetCrouchButtonPressed))
    (Utilities|FlowControl|Gate true
      (:Exit
        (Pawn|Input|AddMovementInput (Math|Vector|GetForwardVector (Math|Rotator|MakeRotator 0.0 0.0 (.Yaw (Math|Rotator|BreakRotator (Pawn|GetControlRotation :!class /Script/Engine.Pawn))))) 1.0 false)))))

(event EventTick
  (params (DeltaSeconds :type Float%20%28single-precision%29))
  ;[1 1 1] Tick Event (Sprint and Stop aming while sprinting)
  (CallFunction|Sprint)
  (CallFunction|StopAimingWhileSprinting))

(event Input|AxisEvents|InputAxisTurn
  (params (AxisValue :type Float%20%28single-precision%29))
  ;[1 1 1] MouseControl
  (Pawn|Input|AddControllerYawInput AxisValue))

(event Input|AxisEvents|InputAxisLookUp
  (params (AxisValue :type Float%20%28single-precision%29))
  ;[1 1 1] MouseControl
  (Pawn|Input|AddControllerPitchInput AxisValue))

(event Input|AxisEvents|InputAxisMoveForward
  (params (AxisValue :type Float%20%28single-precision%29))
  ;[1 1 1] Movement ( AWSD or Joystick)
  (if (not (Variables|Default|GetSprintButtonPressed))
    (Pawn|Input|AddMovementInput (Math|Vector|GetForwardVector (Math|Rotator|MakeRotator 0.0 0.0 (.Yaw (Math|Rotator|BreakRotator (Pawn|GetControlRotation :!class /Script/Engine.Pawn))))) (.X (Math|Vector|BreakVector (Math|Vector|Normalize (Math|Vector|MakeVector AxisValue (stale Input|AxisEvents|InputAxisMoveRight AxisValue) 0.0)))) false)))

(event Input|AxisEvents|InputAxisMoveRight
  (params (AxisValue :type Float%20%28single-precision%29))
  ;[1 1 1] Movement ( AWSD or Joystick)
  (if (not (Variables|Default|GetSprintButtonPressed))
    (Pawn|Input|AddMovementInput (Math|Vector|GetRightVector (Math|Rotator|MakeRotator 0.0 0.0 (.Yaw (Math|Rotator|BreakRotator (Pawn|GetControlRotation :!class /Script/Engine.Pawn))))) (.Y (Math|Vector|BreakVector (Math|Vector|Normalize (Math|Vector|MakeVector (stale Input|AxisEvents|InputAxisMoveForward AxisValue) AxisValue 0.0)))) false)))

(event Input|KeyboardEvents|LeftCtrl
  (params (Key :type Key%20Structure))
  (bind _mesh (Variables|Character|GetMesh))
  (bind _rightmousebuttonpressed (Variables|Default|GetRightMouseButtonPressed))
  ;[1 1 1] Crouch
  (:Pressed
    (Variables|Default|SetCrouchButtonPressed true)
    (Character|Crouch)
    (if _rightmousebuttonpressed
      (Animation|Montage|PlayMontage _mesh "/Game/TPS/M_TPS_WeaponHoldCrouch.M_TPS_WeaponHoldCrouch")))
  (:Released
    (Variables|Default|SetCrouchButtonPressed false)
    (Character|UnCrouch)
    (if _rightmousebuttonpressed
      (Animation|Montage|PlayMontage _mesh "/Game/TPS/M_TPS_WeaponHoldNormal.M_TPS_WeaponHoldNormal"))))

(event Input|MouseEvents|RightMouseButton
  (params (Key :type Key%20Structure))
  (bind _mesh (Variables|Character|GetMesh))
  ;[1 1 1] Aiming( Normal/Crouching)
  (:Pressed
    (if (not (Variables|Default|GetSprintButtonPressed))
      (Variables|Default|SetRightMouseButtonPressed true)
      (if (Variables|Default|GetCrouchButtonPressed)
        (Animation|Montage|PlayMontage _mesh "/Game/TPS/M_TPS_WeaponHoldCrouch.M_TPS_WeaponHoldCrouch")
        (else
          (Animation|Montage|PlayMontage _mesh "/Game/TPS/M_TPS_WeaponHoldNormal.M_TPS_WeaponHoldNormal")))))
  (:Released
    (if (Variables|Default|GetCrouchButtonPressed)
      (Animation|StopAnimMontage "/Game/TPS/M_TPS_WeaponHoldCrouch.M_TPS_WeaponHoldCrouch")
      (else
        (Animation|StopAnimMontage "/Game/TPS/M_TPS_WeaponHoldNormal.M_TPS_WeaponHoldNormal")))))

(event Input|KeyboardEvents|LeftShift
  (params (Key :type Key%20Structure))
  (bind _charactermovement (Variables|Character|GetCharacterMovement))
  ;[1 1 1] Sprint
  (:Pressed
    (Variables|Default|SetSprintButtonPressed true)
    (Variables|/Script/Engine.CharacterMovementComponent|SetMaxWalkSpeed _charactermovement 9e+02)
    (Utilities|FlowControl|Gate true) ; enters at Open
  )
  (:Released
    (Variables|Default|SetSprintButtonPressed false)
    (Variables|/Script/Engine.CharacterMovementComponent|SetMaxWalkSpeed _charactermovement 6e+02)
    (Utilities|FlowControl|Gate true) ; enters at Close
  ))

(event Input|KeyboardEvents|C
  (params (Key :type Key%20Structure))
  ;[1 1 1] Prone
  (:Pressed
    (Variables|Default|SetProneButtonPressed true))
  (:Released
    (Variables|Default|SetProneButtonPressed false)))

(fn ConstructionScript)